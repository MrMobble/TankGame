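; Tank Blueprint that provides physics helper functions for point velocity and braking.
; CalcVelo finds the world-space velocity at a given point on TankBase by combining linear velocity with angular velocity crossed with the offset from the center of mass, computed in local space.
; ApplyBrake reduces an angular velocity toward zero by brake ratio, brake force and frame time, stopping at zero to avoid reversing direction.
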(fn ConstructionScript)

(fn CalcVelo
  (params (Vector :type Vector :default "0, 0, 0"))
  (bind _returnvalue (Transformation|GetActorTransform))
  (bind _tankbase (Variables|Default|GetTankBase))
  (bind _returnvalue_2 (Physics|GetPhysicsLinearVelocity _tankbase "None"))
  (bind _returnvalue_3 (Class|PrimitiveComponent|GetPhysicsAngularVelocity _tankbase "None"))
  (return (Math|Transform|TransformDirection (Transformation|GetActorTransform) (+ (Math|Transform|InverseTransformDirection _returnvalue _returnvalue_2) (Math|Vector|CrossProduct (* (Math|Transform|InverseTransformDirection _returnvalue _returnvalue_3) 0.0174532925) (- (Math|Transform|InverseTransformLocation _returnvalue Vector) (Math|Transform|InverseTransformLocation _returnvalue (Physics|GetCenterOfMass (Variables|Default|GetTankBase) "None"))))))))

(fn ApplyBrake
  (params (AngVelIn :type Float%20%28single-precision%29) (BrakeRatio :type Float%20%28single-precision%29))
  (bind _returnvalue (Utilities|Time|GetWorldDeltaSeconds))
  (bind _brakeforce (Variables|Default|GetBrakeForce))
  (bind _returnvalue_2 (* BrakeRatio _brakeforce _returnvalue))
  (Math|Float|CompareFloat (Math|Float|Absolute(Float) AngVelIn) (Math|Float|Absolute(Float) _returnvalue_2)
    (:>
      (LocalVariables|SetNewVel (- AngVelIn (* _returnvalue_2 (Math|Float|Sign(Float) AngVelIn)))))
    (:==
      (LocalVariables|SetNewVel 0.0 :!label _label))
    (:<
      (goto _label)))
  (return (LocalVariables|GetNewVel)))